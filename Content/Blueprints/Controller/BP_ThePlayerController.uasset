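; Player controller that requests character spawning from BP_TheGameMode.
; SpawnCharacters calls SR_SpawnCharacters only on the local controller, with authority and remote branches differing just in their debug print.
; SR_SpawnCharacters, named as a server-side event, casts the game mode and calls its PCSpawnCharacters.
; BeginPlay and the construction script are empty.
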(event Custom|SR_SpawnCharacters
  (bind _asbp_the_game_mode (Utilities|Casting|CastToBP_TheGameMode (Game|GetGameMode)))
  (Class|ThePlayerController|PCSpawnCharacters _asbp_the_game_mode))

(event EventBeginPlay)

(event EventSpawnCharacters
  ;[1 1 1] Setting
  (Networking|SwitchHasAuthority
    (:Authority
      (if (Pawn|IsLocalPlayerController)
        (CallFunction|SRSpawnCharacters)
        (Development|PrintString "Has Authority")))
    (:Remote
      (if (Pawn|IsLocalPlayerController)
        (CallFunction|SRSpawnCharacters)
        (Development|PrintString "Has No Authority")))))

(fn ConstructionScript)